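; BricolageGameMode is the game mode for Bricolage, tracking counts of things done right, done wrong and still undone.
; On BeginPlay it creates the BricolageUI widget and adds it to the viewport.
; Right and wrong actions update the counters and play a Ding or Error sound, while new things raise the undone count.
; When that count reaches MaxPieces, DeathCheck sets IsDead once and plays the UI's DeathFadeIn animation.
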(event EventBeginPlay
  (bind _returnvalue (UserInterface|CreateWidget "/Game/Bricolage/Blueprints/BricolageUI.BricolageUI_C" (Game|GetPlayerController 0)))
  (bind _output_get (Variables|Default|SetMyUI _returnvalue))
  (UserInterface|Viewport|AddtoViewport _output_get 0))

(event EventTick
  (params (DeltaSeconds :type Float%20%28single-precision%29)))

(fn ConstructionScript)

(fn DoSomethingRight
  (Math|Integer|IncrementInt (Variables|Default|GetThingsDidRight)
    (:%20%20
      (Math|Integer|DecrementInt (Variables|Default|GetThingsUndone)
        (:%20%20
          (Audio|PlaySound2D "/Game/Bricolage/Audio/Ding.Ding" 1.0 1.0 0.0 0 0))))))

(fn DoSomethingWrong
  (Math|Integer|IncrementInt (Variables|Default|GetThingsDidWrong)
    (:%20%20
      (Math|Integer|DecrementInt (Variables|Default|GetThingsUndone)
        (:%20%20
          (Audio|PlaySound2D "/Game/Bricolage/Audio/Error.Error" 1.0 1.0 0.0 0 0))))))

(fn NewThingsCome
  (Math|Integer|IncrementInt (Variables|Default|GetThingsUndone)
    (:%20%20
      (CallFunction|DeathCheck))))

(fn DeathCheck
  (bind _myui (Variables|Default|GetMyUI))
  (if (and (>= (Variables|Default|GetThingsUndone) (Variables|Default|GetMaxPieces)) (Math|Boolean|Equal(Boolean) (Variables|Default|GetIsDead) false))
    (Variables|Default|SetIsDead true)
    (UserInterface|Animation|PlayAnimation _myui (Variables|/Game/Bricolage/Blueprints/BricolageUI.BricolageUI_C|GetDeathFadeIn _myui) 0.0 1 "Forward" 1.0)))