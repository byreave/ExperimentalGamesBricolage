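; Playground is a shape-sorting actor with solver trigger components for spheres, cones and cubes.
; On BeginPlay it caches the BricolageGameMode.
; Each solver's begin overlap casts the incoming actor to its matching shape class (two sphere solvers, one triangular for cones, one box for cubes) and calls DoSomethingRight or DoSomethingWrong on the game mode.
; The overlapping actor is then destroyed either way.
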(event OnComponentBeginOverlap(SphereSolver)
  (params (OverlappedComponent :type Primitive%20Component%20Object%20Reference) (OtherActor :type Actor%20Object%20Reference) (OtherComp :type Primitive%20Component%20Object%20Reference) (OtherBodyIndex :type Integer) (bFromSweep :type Boolean) (SweepResult :type Hit%20Result%20Structure%20%28by%20ref%29))
  (bind _mygamemode (Variables|Default|GetMyGameMode))
  (Utilities|Casting|CastToSphereObject OtherActor
    (:then
      (Default|DoSomethingRight _mygamemode))
    (:CastFailed
      (Default|DoSomethingWrong _mygamemode)))
  (Actor|DestroyActor OtherActor))

(event OnComponentBeginOverlap(SphereSolver2)
  (params (OverlappedComponent :type Primitive%20Component%20Object%20Reference) (OtherActor :type Actor%20Object%20Reference) (OtherComp :type Primitive%20Component%20Object%20Reference) (OtherBodyIndex :type Integer) (bFromSweep :type Boolean) (SweepResult :type Hit%20Result%20Structure%20%28by%20ref%29))
  (bind _mygamemode (Variables|Default|GetMyGameMode))
  (Utilities|Casting|CastToSphereObject OtherActor
    (:then
      (Default|DoSomethingRight _mygamemode))
    (:CastFailed
      (Default|DoSomethingWrong _mygamemode)))
  (Actor|DestroyActor OtherActor))

(event OnComponentBeginOverlap(TriangularSolver)
  (params (OverlappedComponent :type Primitive%20Component%20Object%20Reference) (OtherActor :type Actor%20Object%20Reference) (OtherComp :type Primitive%20Component%20Object%20Reference) (OtherBodyIndex :type Integer) (bFromSweep :type Boolean) (SweepResult :type Hit%20Result%20Structure%20%28by%20ref%29))
  (bind _mygamemode (Variables|Default|GetMyGameMode))
  (Utilities|Casting|CastToConeObject OtherActor
    (:then
      (Default|DoSomethingRight _mygamemode))
    (:CastFailed
      (Default|DoSomethingWrong _mygamemode)))
  (Actor|DestroyActor OtherActor))

(event OnComponentBeginOverlap(BoxSolver)
  (params (OverlappedComponent :type Primitive%20Component%20Object%20Reference) (OtherActor :type Actor%20Object%20Reference) (OtherComp :type Primitive%20Component%20Object%20Reference) (OtherBodyIndex :type Integer) (bFromSweep :type Boolean) (SweepResult :type Hit%20Result%20Structure%20%28by%20ref%29))
  (bind _mygamemode (Variables|Default|GetMyGameMode))
  (Utilities|Casting|CastToCubeObject OtherActor
    (:then
      (Default|DoSomethingRight _mygamemode))
    (:CastFailed
      (Default|DoSomethingWrong _mygamemode)))
  (Actor|DestroyActor OtherActor))

(event EventBeginPlay
  (bind _asbricolage_game_mode (Utilities|Casting|CastToBricolageGameMode (Game|GetGameMode)))
  (Variables|Default|SetMyGameMode _asbricolage_game_mode))

(event Collision|EventActorBeginOverlap
  (params (OtherActor :type Actor%20Object%20Reference)))

(event EventTick
  (params (DeltaSeconds :type Float%20%28single-precision%29)))

(fn ConstructionScript)